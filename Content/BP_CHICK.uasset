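; Player-controlled chicken Character that moves in hops along four directions.
; Directional inputs store a facing and swap in a matching static mesh, while the jump input triggers the hop.
; On jump, the stored facing sets an X or Y step that Tick applies as a frame-rate-dependent local offset until a fixed delay clears it and stops jumping.
; Tick also feeds max jump height into vertical movement input.
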(event EventBeginPlay)

(event Collision|EventActorBeginOverlap
  (params (OtherActor :type Actor%20Object%20Reference)))

(event EventTick
  (params (DeltaSeconds :type Float%20%28single-precision%29))
  (Class|Pawn|ConsumeMovementInputVector)
  (Pawn|Input|AddMovementInput (Math|Vector|MakeVector 0.0 0.0 (Class|CharacterMovementComponent|GetMaxJumpHeightwithJumpTime (Variables|Character|GetCharacterMovement))) 1.0 false)
  (Transformation|AddActorLocalOffset (Math|Vector|MakeVector (Variables|Default|GetmoveX) (Variables|Default|GetmoveY) 0.0) false false))

(event EventOnJumped
  (bind _output_get (Variables|Default|Setdirection (Variables|Default|Getdirection)))
  (switch int _output_get
    (:0
      (Variables|Default|SetmoveX 1.0))
    (:1
      (Variables|Default|SetmoveY 1.0))
    (:2
      (Variables|Default|SetmoveY -1.0))
    (:3
      (Variables|Default|SetmoveX -1.0)))
  (Utilities|FlowControl|Delay 0.85)
  (Variables|Default|SetmoveX 0.0)
  (Variables|Default|SetmoveY 0.0)
  (Character|StopJumping))

(event Input|ActionEvents|InputActionmoveRight
  (params (Key :type Key%20Structure :default "None"))
  (:Pressed
    (Variables|Default|Setdirection 1)
    (Components|StaticMesh|SetStaticMesh (Variables|Default|Getchicken%20mesh) "/Game/D_Chicken.D_Chicken")))

(event Input|ActionEvents|InputActionjumping
  (params (Key :type Key%20Structure :default "None"))
  (:Pressed
    (Character|Jump)))

(event Input|ActionEvents|InputActionmoveForward
  (params (Key :type Key%20Structure :default "None"))
  (:Pressed
    (Variables|Default|Setdirection 0)
    (Components|StaticMesh|SetStaticMesh (Variables|Default|Getchicken%20mesh) "/Game/W_Chicken.W_Chicken")))

(event Input|ActionEvents|InputActionmoveLeft
  (params (Key :type Key%20Structure :default "None"))
  (:Pressed
    (Variables|Default|Setdirection 2)
    (Components|StaticMesh|SetStaticMesh (Variables|Default|Getchicken%20mesh) "/Game/A_Chicken.A_Chicken")))

(event Input|ActionEvents|InputActionmoveBackward
  (params (Key :type Key%20Structure :default "None"))
  (:Pressed
    (Variables|Default|Setdirection 3)
    (Components|StaticMesh|SetStaticMesh (Variables|Default|Getchicken%20mesh) "/Game/S_Chicken.S_Chicken")))

(fn ConstructionScript)