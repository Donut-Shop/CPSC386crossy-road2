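; Spawner actor that lays a chain of Ground land segments at BeginPlay, starting at the player pawn's location.
; Each new segment spawns at the previous one's SpawnPoint, becomes NewestLand and receives a reference back to the spawner.
; An initial loop alternates two grass meshes via FlipFlop, but SpawnLandAtSpawnPoint calls RandomizeLandMesh on that segment before extending.
; A second loop adds more randomized segments.
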(event EventBeginPlay
  (CallFunction|SpawnInitialGrass))

(event Collision|EventActorBeginOverlap
  (params (OtherActor :type Actor%20Object%20Reference)))

(event EventTick
  (params (DeltaSeconds :type Float%20%28single-precision%29)))

(fn ConstructionScript)

(fn SpawnLand
  (params (SpawnLocation :type Vector))
  (bind _returnvalue (Game|SpawnActorfromClass "/Game/landscape_bps/ground/ground.ground_C" (Math|Transform|MakeTransform SpawnLocation "0, 0, 0" "1,1,1") "Undefined" 0 0))
  (bind _output_get (Variables|Default|SetNewestLand _returnvalue))
  (Variables|/Game/landscape_bps/ground/ground.ground_C|SetLandSpawner _output_get self))

(fn SpawnLandatSpawnPoint
  (Default|RandomizeLandMesh (Variables|Default|GetNewestLand))
  (CallFunction|SpawnLand (Transformation|GetWorldLocation (Variables|/Game/landscape_bps/ground/ground.ground_C|GetSpawnPoint (Variables|Default|GetNewestLand)))))

(fn SpawnInitialGrass
  (bind _newestland (Variables|Default|GetNewestLand))
  (for _index (range 0 5)
    (Utilities|FlowControl|FlipFlop
      (:A
        (Components|StaticMesh|SetStaticMesh (Variables|/Game/landscape_bps/ground/ground.ground_C|GetGroundMesh _newestland) "/Game/landscape_bps/ground/grass.grass")
        (Utilities|IsValid (Variables|Default|GetNewestLand)
          (:Is%20Valid
            (CallFunction|SpawnLandatSpawnPoint))
          (:Is%20Not%20Valid
            (CallFunction|SpawnLand (Transformation|GetActorLocation (Game|Player|GetPlayerPawn 0))))))
      (:B
        (Components|StaticMesh|SetStaticMesh (Variables|/Game/landscape_bps/ground/ground.ground_C|GetGroundMesh _newestland) "/Game/landscape_bps/ground/grass2.grass2")
        (Utilities|IsValid (Variables|Default|GetNewestLand)
          (:Is%20Valid
            (CallFunction|SpawnLandatSpawnPoint))
          (:Is%20Not%20Valid
            (CallFunction|SpawnLand (Transformation|GetActorLocation (Game|Player|GetPlayerPawn 0))))))))
  (for _index_2 (range 0 13)
    (Default|RandomizeLandMesh (Variables|Default|GetNewestLand))
    (CallFunction|SpawnLandatSpawnPoint)))